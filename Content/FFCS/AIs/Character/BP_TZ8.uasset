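; BP_TZ8 is an AI enemy character that wakes on player proximity and targets the player through perception.
; Player overlap with its Box tells its DT_TZ8 controller to run its behavior.
; When perception senses the player, it clears the target-check timer, registers itself with the player's AC_AIDirector component and writes the player to the TargetActor blackboard key.
; Nothing in this graph handles losing sight of the player.
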(event `self.AIPerception.OnTargetPerceptionUpdated`
  (params (Actor :type "Actor Object Reference") (Stimulus :type "AIStimulus Structure"))
  (bind _returnvalue (`self.GetComponentByClass` Actor "/Game/FFCS/Blueprints/AC_AIDirector.AC_AIDirector_C"))
  (if (== Actor (`GameplayStatics.GetPlayerCharacter` 0))
    (if (`.bSuccessfullySensed` (break `AIStimulus` Stimulus))
      (`KismetSystemLibrary.K2_ClearAndInvalidateTimerHandle` (`self.TargetCheckerTH`))
      (`/Engine/EditorBlueprintResources/StandardMacros.IsValid` _returnvalue
        (:`Is Valid`
          (`/Game/FFCS/Blueprints/AC_AIDirector.AddEnemy` _returnvalue self))
        (:`Is Not Valid`
          _))
      (`BlackboardComponent.SetValueAsObject` (`AIBlueprintHelperLibrary.GetBlackboard` null) "TargetActor" Actor))))

(event `self.Box.OnComponentBeginOverlap`
  (params (OverlappedComponent :type "PrimitiveComponent Object Reference") (OtherActor :type "Actor Object Reference") (OtherComp :type "PrimitiveComponent Object Reference") (OtherBodyIndex :type Integer) (bFromSweep :type Boolean) (SweepResult :type "HitResult Structure (by ref)"))
  (if (== OtherActor (`GameplayStatics.GetPlayerPawn` 0))
    (bind _asdt_tz8 (cast `/Game/FFCS/AIs/AIController/DT_TZ8` (`self.GetController`)))
    (`/Game/FFCS/AIs/AIController/DT_TZ8.RunBehavior` _asdt_tz8)))

(fn `UserConstructionScript`
  (`parent.UserConstructionScript`))