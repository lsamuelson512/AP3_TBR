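; BP_ChargedProjectile is a charged shot associated with the TZ8 character that damages actors using the free-flow combat component.
; On spawn, a timeline scales up its sphere, then launches it along TZ8's forward direction with a slight downward tilt.
; Hits ignore BP_TZ8; any other hit destroys it, first triggering a forward hit montage with damage on actors that have AC_FreeFlow.
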(event `self.ReceiveBeginPlay`
  (bind (_returnvalue_x _returnvalue_y) (`KismetMathLibrary.BreakVector` (`SceneComponent.GetForwardVector` (`Character.CapsuleComponent` (`self.TZ8Ref`)))))
  (`KismetSystemLibrary.Delay` 0.0)
  (bind (_direction _newtrack_0) (`Timeline|Increase Size`)
    (:`Update`
      (bind _returnvalue (`KismetMathLibrary.Lerp` _newtrack_0 3.0))
      (`SceneComponent.SetWorldScale3D` (`self.Sphere`) (`KismetMathLibrary.MakeVector` _returnvalue _returnvalue _returnvalue)))
    (:`Finished`
      (set `MovementComponent.Velocity` (* (`KismetMathLibrary.MakeVector` _returnvalue_x _returnvalue_y -0.2) 1000.0) (`self.ProjectileMovement`)))))

(event `self.ReceiveHit`
  (params (MyComp :type "PrimitiveComponent Object Reference") (Other :type "Actor Object Reference") (OtherComp :type "PrimitiveComponent Object Reference") (bSelfMoved :type Boolean) (HitLocation :type "Vector Structure") (HitNormal :type "Vector Structure") (NormalImpulse :type "Vector Structure") (Hit :type "HitResult Structure (by ref)"))
  (bind _returnvalue (`self.GetComponentByClass` Other "/Script/AP3_TBR.AC_FreeFlow"))
  (if (!= Other "/Game/FFCS/AIs/Character/BP_TZ8.BP_TZ8")
    (`/Engine/EditorBlueprintResources/StandardMacros.IsValid` _returnvalue
      (:`Is Valid`
        (`AC_FreeFlow.HitDirection` _returnvalue self)
        (`AC_FreeFlow.PlayHitMontage` _returnvalue "Fwd" 6.0)
        (`self.K2_DestroyActor`) ; Then destroy this projectile
      )
      (:`Is Not Valid`
        (`self.K2_DestroyActor`)))))

(fn `UserConstructionScript`)