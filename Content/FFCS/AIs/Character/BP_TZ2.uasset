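; BP_TZ2 is an AI enemy that acquires the player as its target through perception.
; On sensing the player, it clears the TargetCheckerTH timer, registers with the player's AC_AIDirector component and writes the player to the TargetActor blackboard key.
; CheckIfTargetLost unregisters it from the target's director and clears that key.
; Nothing here starts the timer, calls that function or handles losing sight.
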(event `self.AIPerception.OnTargetPerceptionUpdated`
  (params (Actor :type "Actor Object Reference") (Stimulus :type "AIStimulus Structure"))
  (bind _returnvalue (`self.GetComponentByClass` Actor "/Game/FFCS/Blueprints/AC_AIDirector.AC_AIDirector_C"))
  (if (== Actor (`GameplayStatics.GetPlayerCharacter` 0))
    (if (`.bSuccessfullySensed` (break `AIStimulus` Stimulus))
      (`KismetSystemLibrary.K2_ClearAndInvalidateTimerHandle` (`self.TargetCheckerTH`))
      (`/Engine/EditorBlueprintResources/StandardMacros.IsValid` _returnvalue
        (:`Is Valid`
          (`/Game/FFCS/Blueprints/AC_AIDirector.AddEnemy` _returnvalue self))
        (:`Is Not Valid`
          _))
      (`BlackboardComponent.SetValueAsObject` (`AIBlueprintHelperLibrary.GetBlackboard` null) "TargetActor" Actor))))

(fn `CheckIfTargetLost`
  (bind _returnvalue (`BlackboardComponent.GetValueAsObject` (`AIBlueprintHelperLibrary.GetBlackboard` null) "TargetActor"))
  (bind _returnvalue_2 (`self.GetComponentByClass` (cast `Character` _returnvalue :!pure true) "/Game/FFCS/Blueprints/AC_AIDirector.AC_AIDirector_C"))
  (`/Engine/EditorBlueprintResources/StandardMacros.IsValid` _returnvalue
    (:`Is Valid`
      (`/Engine/EditorBlueprintResources/StandardMacros.IsValid` _returnvalue_2
        (:`Is Valid`
          (`/Game/FFCS/Blueprints/AC_AIDirector.RemoveEnemy` _returnvalue_2 self))
        (:`Is Not Valid`
          _))
      (`BlackboardComponent.SetValueAsObject` (`AIBlueprintHelperLibrary.GetBlackboard` null) "TargetActor" null))))

(fn `UserConstructionScript`)