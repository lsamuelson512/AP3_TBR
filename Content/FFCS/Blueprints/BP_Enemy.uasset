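; BP_Enemy is an enemy character Blueprint with helper functions for choosing a pounce target; no pounce action or caller appears here.
; EnemiesInRange gathers overlapping Pawns in a sphere, excluding itself.
; DotProductEnemy scores an actor's direction against a product of last movement input and control-yaw forward and right vectors.
; BestEnemyPounce compares those scores, but never updates its threshold, returning the last candidate above -1.
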(fn `BestEnemyPounce`
  (params (Enemies :type "Array of Actor Object Reference"))
  (returns (Enemy :type "Actor Object Reference"))
  (locals (Dot :type "Float (double-precision)" :default -1.0) (BestEnemy :type "Actor Object Reference"))
  (bind _dot (`local.Dot`))
  (set `local.Dot` -1.0)
  (for _array_element Enemies
    (bind _dot_2 (`self.DotProductEnemy` _array_element))
    (if (> _dot_2 _dot)
      (set `local.BestEnemy` _array_element)
      (set `local.Dot` _dot)))
  (return (`local.BestEnemy`)))

(fn `DotProductEnemy`
  (params (Enemy :type "Actor Object Reference"))
  (returns (Dot :type "Float (double-precision)"))
  (bind (_returnvalue_roll _returnvalue_pitch _returnvalue_yaw) (`KismetMathLibrary.BreakRotator` (`self.GetControlRotation`)))
  (bind _returnvalue (`KismetMathLibrary.MakeRotator` 0.0 0.0 _returnvalue_yaw))
  (return (`KismetMathLibrary.Dot_VectorVector` (`KismetMathLibrary.Normal` (- (`self.K2_GetActorLocation` Enemy) (`self.K2_GetActorLocation`))) (`KismetMathLibrary.Normal` (* (`PawnMovementComponent.GetLastInputVector` (`self.CharacterMovement`)) (`KismetMathLibrary.GetForwardVector` _returnvalue) (`KismetMathLibrary.GetRightVector` _returnvalue))))))

(fn `EnemiesInRange`
  (params (Range :type "Float (double-precision)"))
  (returns (Targets :type "Array of Actor Object Reference"))
  (bind (_outactors _returnvalue) (`KismetSystemLibrary.SphereOverlapActors` (`self.K2_GetActorLocation`) Range (`|MakeArray` "ObjectTypeQuery3" :!type "EObjectTypeQuery Enum") null (`|MakeArray` self :!type "Actor Object Reference")))
  (if _returnvalue
    (return _outactors)))

(fn `UserConstructionScript`)