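; AC_FreeFlow is a component that holds shared player combat state, apparently for a free-flow combat system.
; It stores the current enemy and a player state gameplay tag, each exposed through a setter and getter.
; Setting the tag also prints its name for debugging, and the component runs no BeginPlay or Tick logic of its own.
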(fn `GetCurrEnemy`
  (returns (CurrEnemy :type "Actor Object Reference"))
  (return (`self.CurrEnemy`)))

(fn `GetCurrentTag`
  (returns (Tag :type "GameplayTag Structure"))
  (return (`self.PlayerStateTag`)))

(fn `SetCurrEnemy`
  (params (CurrEnemy :type "Actor Object Reference"))
  (set `self.CurrEnemy` CurrEnemy))

(fn `SetTag`
  (params (PlayerStateTag :type "GameplayTag Structure"))
  (bind _output_get (set `self.PlayerStateTag` PlayerStateTag))
  (`KismetSystemLibrary.PrintString` (`KismetStringLibrary.Conv_NameToString` (`BlueprintGameplayTagLibrary.GetTagName` _output_get))))